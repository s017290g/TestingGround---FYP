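; EnemyTile is the opponent's target in a card game, showing its Health on a TextRender and taking attacks when released on.
; If no taunts are in play, a release applies the game mode's Card1Attack as damage; otherwise it prints a refusal.
; LoseHealth updates the text, then prints a player win at zero or below, or clears Card1Attack.
; AddHealth is empty, and board-scanning logic for card effects is disconnected.
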(event `self.ReceiveBeginPlay`
  ;[1 1 1] Event Start
  (`TextRenderComponent.K2_SetText` (`self.TextRender`) (`KismetTextLibrary.Conv_IntToText` (`self.Health`))))

(event `self.ReceiveActorOnReleased`
  (params (ButtonReleased :type "Key Structure"))
  ;[1 1 1] Event Start
  (if (<= (`self.Number of Taunts in play`) 0)
    (`KismetSystemLibrary.PrintString` "Hello")
    (bind _ascard_game_mode (cast `/Game/Blueprints/GameState/Card_GameMode` (`GameplayStatics.GetGameMode`)))
    (`self.Lose Health` (`/Game/Blueprints/GameState/Card_GameMode.Card1 Attack` _ascard_game_mode))
    (else
      (`KismetSystemLibrary.PrintString` "You can not attack until taunt is dead"))))

(event `Lose Health`
  (params (`Damage Taken` :type Integer))
  (bind _textrender (`self.TextRender`))
  (bind _returnvalue (`KismetTextLibrary.Conv_IntToText` (`self.Health`)))
  (bind _output_get (set `self.Health` (- (`self.Health`) `Damage Taken`)))
  (if (<= _output_get 0)
    (`TextRenderComponent.K2_SetText` _textrender _returnvalue)
    (`KismetSystemLibrary.PrintString` "Player wins")
    (else
      (`TextRenderComponent.K2_SetText` _textrender _returnvalue)
      (set `/Game/Blueprints/GameState/Card_GameMode.Card1 Attack` 0 (stale `self.ReceiveActorOnReleased` _ascard_game_mode)))))

(event `Add Health`)

(fn `UserConstructionScript`)