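; Board controller that plays a dragged card onto the board when Player 1 has enough mana.
; BeginPlay caches enemy and board tiles, also sorting the latter by player index.
; OnCardDrag opens a gate on Tick, which deducts mana, then snaps the card to the first unoccupied tile of either board and links them.
; Placement or insufficient mana closes the gate; no collision test runs, and ZoneCheck is empty.
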(event `self.ReceiveBeginPlay`
  ;[1 1 1] Get Enemy Tile
  (`|ExecutionSequence`
    (:`then_0`
      (bind _outactors (`GameplayStatics.GetAllActorsOfClass` "/Game/Blueprints/EnemyTile.EnemyTile_C"))
      (bind _output_get (set `self.Enemy` _outactors))
      (set `self.EnemyRef` (`|GetArrayItem` _output_get)))
    (:`then_1`
      (bind _outactors_2 (`GameplayStatics.GetAllActorsOfClass` "/Game/Blueprints/Board/BoardTile.BoardTile_C"))
      (bind _output_get_2 (set `self.Tiles` _outactors_2))
      (for _array_element _output_get_2
        (if (== (`/Game/Blueprints/Board/BoardTile.Player Index` _array_element) 0)
          (set `self.Player 1 Board` (`|MakeArray` _array_element))
          (else
            (set `self.Player 2 Board` (`|MakeArray` _array_element))))))))

(event `self.ReceiveTick`
  (params (DeltaSeconds :type "Float (single-precision)"))
  (bind _tiles (`self.Tiles`))
  (bind _cardoverlapped (`self.CardOverlapped`))
  (bind _asplayer_1pawn (cast `/Game/Models/Pawn/Player1Pawn` (`GameplayStatics.GetPlayerPawn` 0) :!pure true))
  (`/Engine/EditorBlueprintResources/StandardMacros.Gate` true :!label _label
    (:`Exit`
      (bind _output_get (set `self.CardOverlapped` (stale `On Card Drag` CardOverlappedRef)))
      (if (<= (`/Game/Blueprints/Cards/BaseCard.ManaCost_Value` _output_get) (`/Game/Models/Pawn/Player1Pawn.Mana` (cast `/Game/Models/Pawn/Player1Pawn` (`GameplayStatics.GetPlayerPawn` 0) :!pure true)))
        (set `/Game/Models/Pawn/Player1Pawn.Mana` (- (`/Game/Models/Pawn/Player1Pawn.Mana` _asplayer_1pawn) (`/Game/Blueprints/Cards/BaseCard.ManaCost_Value` _output_get)) _asplayer_1pawn)
        (for (_ _array_index) _tiles :!label _label_2
          (bind _output (`|GetArrayItem` _tiles _array_index))
          (if (not (`/Game/Blueprints/Board/BoardTile.IsOccupied` _output))
            (`|ExecutionSequence`
              (:`then_0`
                (`self.Break`))
              (:`then_1`
                (set `/Game/Blueprints/Board/BoardTile.IsOccupied` true _output)
                (`self.K2_SetActorTransform` _cardoverlapped (`KismetMathLibrary.MakeTransform` (`self.K2_GetActorLocation` _output) (struct :`Roll` -90.0) (0.4 0.4 0.4)) false false)
                (set `/Game/Blueprints/Cards/BaseCard.StateSelection` "NewEnumerator2" _cardoverlapped)
                (`self.OnCardDragRelease`))
              (:`then_2`
                (set `/Game/Blueprints/Cards/BaseCard.Board Tile` _output _cardoverlapped)))))
        (else
          (`self.OnCardDragRelease`))))))

(event `On Card Drag`
  (params (CardOverlappedRef :type "/Game/Blueprints/Cards/BaseCard Object Reference"))
  (goto _label :!via `Open`))

(event `Break`
  (goto _label_2 :!via `Break`))

(event `OnCardDragRelease`
  (goto _label :!via `Close`))

(fn `UserConstructionScript`)

(fn `ZoneCheck`
  (params (ZoneLoc :type "Vector Structure") (NewParam1 :type "Vector Structure" :default (0.0 0.0 0.0))))