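; BoardTile is a board slot actor that lets the player play a card by releasing it over the tile.
; Box overlap opens a gate so Tick watches for the mouse release, then checks and deducts Player1Pawn mana.
; If unoccupied, the tile snaps the card into place, shuts off its hover and click input, and claims it.
; Taunt cards also increment the taunt count on the first EnemyTile found at BeginPlay.
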(event `self.ReceiveBeginPlay`
  ;[1 1 1] Get Enemy Tile
  (bind _outactors (`GameplayStatics.GetAllActorsOfClass` "/Game/Blueprints/EnemyTile.EnemyTile_C"))
  (bind _output_get (set `self.Enemy` _outactors))
  (set `self.EnemyRef` (`|GetArrayItem` _output_get))
  (set `self.PlayerInt` (`self.PlayerInt`)))

(event `self.ReceiveTick`
  (params (DeltaSeconds :type "Float (single-precision)"))
  (bind _enemyref (`self.EnemyRef`))
  (bind _asplayer_1pawn (cast `/Game/Models/Pawn/Player1Pawn` (`GameplayStatics.GetPlayerPawn` 0) :!pure true))
  (`/Engine/EditorBlueprintResources/StandardMacros.Gate` true :!label _label
    (:`Exit`
      (bind _output_get (set `self.CardOverlapped` (`|MakeArray` (stale `self.Box.OnComponentBeginOverlap` OtherActor))))
      (bind _output (`|GetArrayItem` _output_get))
      (bind _card (`self.Is Mouse Released Over Overlap` _output)
        (:`Output`
          (if (<= (`/Game/Blueprints/Cards/BaseCard.ManaCost_Value` (cast `/Game/Blueprints/Cards/BaseCard` _output :!pure true)) (`/Game/Models/Pawn/Player1Pawn.Mana` (cast `/Game/Models/Pawn/Player1Pawn` (`GameplayStatics.GetPlayerPawn` 0) :!pure true)))
            (set `/Game/Models/Pawn/Player1Pawn.Mana` (- (`/Game/Models/Pawn/Player1Pawn.Mana` _asplayer_1pawn) (`/Game/Blueprints/Cards/BaseCard.ManaCost_Value` (cast `/Game/Blueprints/Cards/BaseCard` _output :!pure true))) _asplayer_1pawn)
            (if (not (`self.IsOccupied`))
              (set `/Game/Blueprints/Cards/BaseCard.StateSelection` "NewEnumerator2" _card)
              (`self.ZoneCheck` _card (`SceneComponent.K2_GetComponentLocation` (`self.Box`)))
              (set `self.IsOccupied` true)
              (set `/Game/Blueprints/Cards/BaseCard.Board Tile` self _card)
              (switch `/Game/Blueprints/Cards/Card_SpecialEffect` (`/Game/Blueprints/Cards/BaseCard.SpecialEffectEnum` _card)
                (:`NewEnumerator1`
                  (bind _result (`/Engine/EditorBlueprintResources/StandardMacros.IncrementInt` (`/Game/Blueprints/EnemyTile.Number of Taunts in play` _enemyref))
                    (:`  `
                      (set `/Game/Blueprints/EnemyTile.Number of Taunts in play` _result _enemyref))))))))))))

(event `self.Box.OnComponentBeginOverlap`
  (params (OverlappedComponent :type "PrimitiveComponent Object Reference") (OtherActor :type "Actor Object Reference") (OtherComp :type "PrimitiveComponent Object Reference") (OtherBodyIndex :type Integer) (bFromSweep :type Boolean) (SweepResult :type "HitResult Structure (by ref)"))
  (goto _label :!via `Open`))

(event `self.Box.OnComponentEndOverlap`
  (params (OverlappedComponent :type "PrimitiveComponent Object Reference") (OtherActor :type "Actor Object Reference") (OtherComp :type "PrimitiveComponent Object Reference") (OtherBodyIndex :type Integer))
  (goto _label :!via `Close`))

(fn `UserConstructionScript`)

(fn `ZoneCheck`
  (params (`Base Card` :type "/Game/Blueprints/Cards/BaseCard Object Reference") (`Zone Location` :type "Vector Structure"))
  (`self.K2_SetActorTransform` (`|GetArrayItem` (`self.CardOverlapped`)) (`KismetMathLibrary.MakeTransform` `Zone Location` (struct :`Roll` -90.0) (0.6 0.6 0.6)) false false)
  (`/Game/Blueprints/Cards/BaseCard.StopHover` `Base Card`)
  (`/Game/Blueprints/Cards/BaseCard.StopEndHover` `Base Card`)
  (`/Game/Blueprints/Cards/BaseCard.CloseOnClickGate` `Base Card`)
  (`/Game/Blueprints/Cards/BaseCard.CloseOnRelaseGate` `Base Card`))