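; Player board for a card game that snaps a dropped card into the first free of seven zones.
; CollisionZone overlap opens and closes a gate on Tick, which polls the overlapping BaseCard for a mouse release.
; On release it sets the card's state, and ZoneCheck moves, rotates and shrinks it and shuts off its hover and click handling.
; Zone occupancy is tracked by booleans that are only cleared here, never restored.
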(event `self.ReceiveTick`
  (params (DeltaSeconds :type "Float (single-precision)"))
  ;[1 1 1] Rework later
  (`/Engine/EditorBlueprintResources/StandardMacros.Gate` true :!label _label
    (:`Exit`
      (bind _output_get (set `self.CardOverlapped` (stale `self.Collision Zone.OnComponentBeginOverlap` OtherActor)))
      (bind _newparam (`self.IsMouseRelasedOverOverlap` _output_get)
        (:`Output`
          (if (`self.Zone1Empty`)
            (set `/Game/Blueprints/Cards/BaseCard.StateSelection` "NewEnumerator2" _newparam)
            (`self.ZoneCheck` _newparam (`SceneComponent.K2_GetComponentLocation` (`self.Zone 1`)))
            (set `self.Zone1Empty` false)
            (`self.SetActorScale3D` _output_get (0.6 0.6 0.6) :!label _label_2)
            (elif (`self.Zone2Empty`)
              (set `/Game/Blueprints/Cards/BaseCard.StateSelection` "NewEnumerator2" _newparam)
              (`self.ZoneCheck` _newparam (`SceneComponent.K2_GetComponentLocation` (`self.Zone 2`)))
              (set `self.Zone2Empty` false)
              (goto _label_2)
              (elif (`self.Zone3Empty`)
                (set `/Game/Blueprints/Cards/BaseCard.StateSelection` "NewEnumerator2" _newparam)
                (`self.ZoneCheck` _newparam (`SceneComponent.K2_GetComponentLocation` (`self.Zone 3`)))
                (set `self.Zone3Empty` false)
                (goto _label_2)
                (elif (`self.Zone4Empty`)
                  (set `/Game/Blueprints/Cards/BaseCard.StateSelection` "NewEnumerator2" _newparam)
                  (`self.ZoneCheck` _newparam (`SceneComponent.K2_GetComponentLocation` (`self.Zone 4`)))
                  (set `self.Zone4Empty` false)
                  (goto _label_2)
                  (elif (`self.Zone5Empty`)
                    (set `/Game/Blueprints/Cards/BaseCard.StateSelection` "NewEnumerator2" _newparam)
                    (`self.ZoneCheck` _newparam (`SceneComponent.K2_GetComponentLocation` (`self.Zone 5`)))
                    (set `self.Zone5Empty` false)
                    (goto _label_2)
                    (elif (`self.Zone6Empty`)
                      (set `/Game/Blueprints/Cards/BaseCard.StateSelection` "NewEnumerator2" _newparam)
                      (`self.ZoneCheck` _newparam (`SceneComponent.K2_GetComponentLocation` (`self.Zone 6`)))
                      (set `self.Zone6Empty` false)
                      (goto _label_2)
                      (elif (`self.Zone7Empty`)
                        (set `/Game/Blueprints/Cards/BaseCard.StateSelection` "NewEnumerator2" _newparam)
                        (`self.ZoneCheck` _newparam (`SceneComponent.K2_GetComponentLocation` (`self.Zone 7`)))
                        (set `self.Zone7Empty` false)
                        (goto _label_2)
                        (else
                          (`KismetSystemLibrary.PrintString` "No more slots"))))))))))))))

(event `self.Collision Zone.OnComponentBeginOverlap`
  (params (OverlappedComponent :type "PrimitiveComponent Object Reference") (OtherActor :type "Actor Object Reference") (OtherComp :type "PrimitiveComponent Object Reference") (OtherBodyIndex :type Integer) (bFromSweep :type Boolean) (SweepResult :type "HitResult Structure (by ref)"))
  ;[1 1 1] Rework later
  (goto _label :!via `Open`))

(event `self.Collision Zone.OnComponentEndOverlap`
  (params (OverlappedComponent :type "PrimitiveComponent Object Reference") (OtherActor :type "Actor Object Reference") (OtherComp :type "PrimitiveComponent Object Reference") (OtherBodyIndex :type Integer))
  ;[1 1 1] Rework later
  (goto _label :!via `Close`))

(fn `UserConstructionScript`)

(fn `ZoneCheck`
  (params (BaseCard :type "/Game/Blueprints/Cards/BaseCard Object Reference") (ZoneLoc :type "Vector Structure"))
  (`self.K2_SetActorTransform` (`self.CardOverlapped`) (`KismetMathLibrary.MakeTransform` ZoneLoc (struct :`Roll` -90.0) (0.6 0.6 0.6)) false false)
  (`/Game/Blueprints/Cards/BaseCard.StopHover` BaseCard)
  (`/Game/Blueprints/Cards/BaseCard.StopEndHover` BaseCard)
  (`/Game/Blueprints/Cards/BaseCard.CloseOnClickGate` BaseCard)
  (`/Game/Blueprints/Cards/BaseCard.CloseOnRelaseGate` BaseCard))