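; AI board Blueprint for a card game, providing helpers for placing cards into board zones.
; ZoneCheck snaps the overlapped card to a zone location, laid flat and scaled down, then stops hover and closes the click and release gates on the passed BaseCard.
; IsMouseRelasedOverOverlap checks an overlapped card's mouse-release flag, clearing it and returning that card when set.
; BeginPlay and the construction script are empty.
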(event `self.ReceiveBeginPlay`)

(fn `UserConstructionScript`)

(fn `ZoneCheck`
  (params (BaseCard :type "/Game/Blueprints/Cards/BaseCard Object Reference") (ZoneLoc :type "Vector Structure"))
  (`self.K2_SetActorTransform` (`self.CardOverlapped`) (`KismetMathLibrary.MakeTransform` ZoneLoc (struct :`Roll` -90.0) (0.6 0.6 0.6)) false false)
  (`/Game/Blueprints/Cards/BaseCard.StopHover` BaseCard)
  (`/Game/Blueprints/Cards/BaseCard.StopEndHover` BaseCard)
  (`/Game/Blueprints/Cards/BaseCard.CloseOnClickGate` BaseCard)
  (`/Game/Blueprints/Cards/BaseCard.CloseOnRelaseGate` BaseCard))