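; EnemyBoardCollisionCheck1 handles card drags on the board, checking the dragged card's cost against Player1Pawn's mana.
; BeginPlay caches a PlayerTile and all EnemyBoardTiles.
; A Gate opened by OnCardDrag lets Tick deduct the card's cost on every frame, closing when mana is short or the drag is released.
; Logic to snap cards onto free enemy tiles is unwired, and ZoneCheck is empty.
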(event `self.ReceiveBeginPlay`
  ;[1 1 1] Get Enemy Tile
  (`|ExecutionSequence`
    (:`then_0`
      (bind _outactors (`GameplayStatics.GetAllActorsOfClass` "/Game/Blueprints/PlayerTile.PlayerTile_C"))
      (set `self.PlayerRef` (`|GetArrayItem` _outactors)))
    (:`then_1`
      (bind _outactors_2 (`GameplayStatics.GetAllActorsOfClass` "/Game/Blueprints/Board/EnemyBoardTile.EnemyBoardTile_C"))
      (set `self.EnemyTiles` _outactors_2))))

(event `self.ReceiveTick`
  (params (DeltaSeconds :type "Float (single-precision)"))
  (bind _asplayer_1pawn (cast `/Game/Models/Pawn/Player1Pawn` (`GameplayStatics.GetPlayerPawn` 0) :!pure true))
  (`/Engine/EditorBlueprintResources/StandardMacros.Gate` true :!label _label
    (:`Exit`
      (bind _output_get (set `self.CardOverlapped` (stale `On Card Drag` CardOverlappedRef)))
      (if (<= (`/Game/Blueprints/Cards/BaseCard.ManaCost_Value` _output_get) (`/Game/Models/Pawn/Player1Pawn.Mana` (cast `/Game/Models/Pawn/Player1Pawn` (`GameplayStatics.GetPlayerPawn` 0) :!pure true)))
        (set `/Game/Models/Pawn/Player1Pawn.Mana` (- (`/Game/Models/Pawn/Player1Pawn.Mana` _asplayer_1pawn) (`/Game/Blueprints/Cards/BaseCard.ManaCost_Value` _output_get)) _asplayer_1pawn)
        (else
          (`self.OnCardDragRelease`))))))

(event `On Card Drag`
  (params (CardOverlappedRef :type "/Game/Blueprints/Cards/BaseCard Object Reference"))
  (goto _label :!via `Open`))

(event `Break`
  (bind _output (`|GetArrayItem` _))
  (bind _cardoverlapped (`self.CardOverlapped`))
  (bind _enemytiles (`self.EnemyTiles`))
  (for (_ _array_index) _enemytiles :!via `Break`
    (if (not (`/Game/Blueprints/Board/EnemyBoardTile.IsOccupied` (`|GetArrayItem` _enemytiles _array_index)))
      (`|ExecutionSequence`
        (:`then_0`
          (`self.Break`))
        (:`then_1`
          (set `/Game/Blueprints/Board/BoardTile.IsOccupied` true _output)
          (`self.K2_SetActorTransform` _cardoverlapped (`KismetMathLibrary.MakeTransform` (`self.K2_GetActorLocation` _output) (struct :`Roll` -90.0) (0.4 0.4 0.4)) false false)
          (set `/Game/Blueprints/Cards/BaseCard.StateSelection` "NewEnumerator2" _cardoverlapped)
          (`self.OnCardDragRelease`))
        (:`then_2`
          (set `/Game/Blueprints/Cards/BaseCard.Board Tile` _output _cardoverlapped))))))

(event `OnCardDragRelease`
  (goto _label :!via `Close`))

(fn `UserConstructionScript`)

(fn `ZoneCheck`
  (params (ZoneLoc :type "Vector Structure") (NewParam1 :type "Vector Structure" :default (0.0 0.0 0.0))))