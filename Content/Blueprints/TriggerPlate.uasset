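; TriggerPlate is a trigger that draws a card from a shuffled deck when something overlaps its collision.
; On BeginPlay it loads the row names of a card data table into an array and shuffles them.
; Each overlap, gated by a DoOnce that resets on end overlap, looks up the current row, prints its card name and advances the index.
; The bounds check reports an empty deck one card early, leaving the last undrawn.
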(event `self.ReceiveBeginPlay`
  (bind _outrownames (`DataTableFunctionLibrary.GetDataTableRowNames` "/Game/Blueprints/Card_Data_Table.Card_Data_Table"))
  (bind _output_get (set `self.Cards In Deck` _outrownames))
  (`KismetArrayLibrary.Array_Shuffle` _output_get))

(event `self.Collision.OnComponentBeginOverlap`
  (params (OverlappedComponent :type "PrimitiveComponent Object Reference") (OtherActor :type "Actor Object Reference") (OtherComp :type "PrimitiveComponent Object Reference") (OtherBodyIndex :type Integer) (bFromSweep :type Boolean) (SweepResult :type "HitResult Structure (by ref)"))
  (`/Engine/EditorBlueprintResources/StandardMacros.DoOnce` false :!label _label
    (:`Completed`
      (if (>= (`self.Current Array Index`) (- (`KismetArrayLibrary.Array_Length` (`self.Cards In Deck`)) 1))
        (`KismetSystemLibrary.PrintString` "No More Cards In Deck")
        (else
          (`self.Set Card Data` (`|GetArrayItem` (`self.Cards In Deck`) (`self.Current Array Index`)))
          (`/Engine/EditorBlueprintResources/StandardMacros.IncrementInt` (`self.Current Array Index`)))))))

(event `self.Collision.OnComponentEndOverlap`
  (params (OverlappedComponent :type "PrimitiveComponent Object Reference") (OtherActor :type "Actor Object Reference") (OtherComp :type "PrimitiveComponent Object Reference") (OtherBodyIndex :type Integer))
  (goto _label :!via `Reset`))

(event `Set Card Data`
  (params (NewParam :type Name))
  (bind _returnvalue (`|GetDataTableRow` "/Game/Blueprints/Card_Data_Table.Card_Data_Table" NewParam)
    (:`then`
      (`KismetSystemLibrary.PrintString` (`.CardName_11_E12B11F24B5BE2A2B17FC597792A062B` (break `/Game/Blueprints/Card_Data_Struc` _returnvalue))))))

(fn `UserConstructionScript`)