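; DrawManager deals a random hand of cards in front of the player when play begins.
; It gathers every BaseCard actor already in the level, shuffles the array, and teleports the cards in a configured index range into a row.
; The row starts at a fixed world-space offset from the player character and steps by a set spacing, with each card's roll taken from the follow camera's pitch.
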(event `self.ReceiveBeginPlay`
  ;[1 1 1] For the love of all that is holy, change this fucking code
  (bind _outactors (`GameplayStatics.GetAllActorsOfClass` "/Game/Blueprints/Cards/BaseCard.BaseCard_C"))
  (bind _output_get (set `self.AllCards` _outactors))
  (`KismetArrayLibrary.Array_Shuffle` _output_get)
  (set `self.CardStartLoc` (+ (`self.K2_GetActorLocation` (`GameplayStatics.GetPlayerCharacter` 0)) (-150.0 415.0 -50.0)))
  (set `self.CardRotation` (`KismetMathLibrary.MakeRotator` (.pitch (`SceneComponent.K2_GetComponentRotation` (`/Game/ThirdPersonBP/Blueprints/ThirdPersonCharacter.FollowCamera` (cast `/Game/ThirdPersonBP/Blueprints/ThirdPersonCharacter` (`GameplayStatics.GetPlayerCharacter` 0) :!pure true))))))
  (for _index (range (`self.StartingNo`) (+ (`self.EndingNo`) 1))
    (set `self.AmountOfDrawnCards` _index)
    (`self.K2_TeleportTo` (`|GetArrayItem` (`self.AllCards`) (`self.AmountOfDrawnCards`)) (`self.CardStartLoc`) (`self.CardRotation`))
    (set `self.CardStartLoc` (+ (`self.CardStartLoc`) (`self.CardOffsetToNext`)))))

(fn `UserConstructionScript`)