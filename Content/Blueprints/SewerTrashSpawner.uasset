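; Spawner actor that repeatedly creates a SewerTrash actor at its own root transform, ignoring collisions.
; BeginPlay starts a self-repeating loop that spawns the trash, destroys it after a fixed seven-second lifetime, then waits a random interval between two range variables before calling SpawnNewObject again.
; Each cycle destroys its trash before the next spawn, so the spawner keeps at most one piece alive at a time.
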(event `SpawnNewObject`
  (bind _returnvalue (`|SpawnActorFromClass` "/Game/Blueprints/SewerTrash.SewerTrash_C" (`SceneComponent.K2_GetComponentToWorld` (`self.DefaultSceneRoot`)) "AlwaysSpawn" "OverrideRootScale" null null :!label _label))
  (`KismetSystemLibrary.Delay` 7.0)
  (`self.K2_DestroyActor` _returnvalue)
  (`KismetSystemLibrary.Delay` (`KismetMathLibrary.RandomFloatInRange` (`self.MinRandomRange`) (`self.MaxTandomRange`)))
  (`self.SpawnNewObject`))

(event `self.ReceiveBeginPlay`
  (goto _label))

(fn `UserConstructionScript`)