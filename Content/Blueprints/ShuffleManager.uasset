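; ShuffleManager deals randomized card data to the card actors in the level when play begins.
; It reads all row names from the card data table into a deck array and shuffles it.
; It then walks every BaseCard actor, assigning each the next shuffled row through SetCardData until the deck runs out, and prints a debug message when the loop finishes.
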(event `self.ReceiveBeginPlay`
  ;[1 1 1] Shuffle Cards
  (bind _outrownames (`DataTableFunctionLibrary.GetDataTableRowNames` "/Game/Blueprints/Cards/Card_Data_Table.Card_Data_Table"))
  (bind _output_get (set `self.Cards In Deck` _outrownames))
  (`KismetArrayLibrary.Array_Shuffle` _output_get)
  ;[1 1 1] Loop through deck to create random order of cards, with the cards value matching the value given to it in the data table
  (bind _outactors (`GameplayStatics.GetAllActorsOfClass` "/Game/Blueprints/Cards/BaseCard.BaseCard_C"))
  (for _array_element _outactors
    (if (not (>= (`self.Current Array Index`) (`KismetArrayLibrary.Array_Length` (`self.Cards In Deck`))))
      (`/Game/Blueprints/Cards/BaseCard.Set Card Data` _array_element (`|GetArrayItem` (`self.Cards In Deck`) (`self.Current Array Index`)))
      (`/Engine/EditorBlueprintResources/StandardMacros.IncrementInt` (`self.Current Array Index`))))
  (`KismetSystemLibrary.PrintString` "No More Cards"))

(fn `UserConstructionScript`)