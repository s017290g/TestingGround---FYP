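; AI card actor that displays name, attack, defense and mana cost loaded by row from AI_Card_Data_Table.
; StateSelection routes cursor events: in Hand the card enlarges on hover and follows the cursor through gated Tick teleports until released.
; On Board, click and release send the BaseCard under the cursor to Card_GameMode's two combat checks; in Grave, a click opens the Graveyard_Slider widget.
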(event `State Custom Event`
  (switch `/Game/Blueprints/Cards/CardStateEnum` (`self.StateSelection`)
    (:`NewEnumerator1`
      (set `self.OldLoc` (`SceneComponent.K2_GetComponentLocation` (`self.DefaultSceneRoot`))))))

(event `Set Card Data`
  (params (Row :type Name))
  ;[1 1 1] Sets the cards values based on the index value during the loop
  (bind _returnvalue (`|GetDataTableRow` "/Game/Blueprints/Cards/AI_Card_Data_Table.AI_Card_Data_Table" Row)
    (:`then`
      (bind (_cardname _manacost _attackvalue _defensevalue) (break `/Game/Blueprints/Cards/Card_Data_Struc` _returnvalue))
      (set `self.Title_Text` (`KismetTextLibrary.Conv_StringToText` _cardname))
      (set `self.Att_Value` _attackvalue)
      (set `self.Def_Value` _defensevalue)
      (set `self.ManaCost_Value` _manacost)
      (`self.UpdateValues`))))

(event `StopHover`
  ;[1 0.01016 0] Old
  ;;[1 1 1] On Card Hover
)

(event `self.Card.OnBeginCursorOver`
  (params (TouchedComponent :type "PrimitiveComponent Object Reference"))
  ;[1 1 1] On start hover
  (switch `/Game/Blueprints/Cards/CardStateEnum` (`self.StateSelection`)
    (:`NewEnumerator1`
      (`self.On Hover`))))

(event `OpenEndOver`
  ;[1 0.01016 0] Old
  ;;[1 1 1] On end hover
)

(event `self.Card.OnEndCursorOver`
  (params (TouchedComponent :type "PrimitiveComponent Object Reference"))
  ;[1 1 1] On end hover
  (switch `/Game/Blueprints/Cards/CardStateEnum` (`self.StateSelection`)
    (:`NewEnumerator1`
      (`KismetSystemLibrary.PrintString` "end hover")
      (`self.End Hover`))))

(event `StopEndHover`
  ;[1 0.01016 0] Old
  ;;[1 1 1] On end hover
)

(event `self.Card.OnClicked`
  (params (TouchedComponent :type "PrimitiveComponent Object Reference") (ButtonPressed :type "Key Structure"))
  (switch `/Game/Blueprints/Cards/CardStateEnum` (`self.StateSelection`)
    (:`NewEnumerator1`
      ;[1 1 1] On Click - In Hand State
      (`/Engine/EditorBlueprintResources/StandardMacros.Gate` false :!label _label
        (:`Exit`
          (set `self.MouseRelased` false)
          (goto _label_2 :!via `Open`))))
    (:`NewEnumerator2`
      (`self.On Click - Boad State`))
    (:`NewEnumerator4`
      (bind _returnvalue (`|CreateWidget` "/Game/Widgets/InGame/Graveyard_Slider.Graveyard_Slider_C"))
      (`UserWidget.AddToViewport` _returnvalue 0))))

(event `self.ReceiveTick`
  (params (DeltaSeconds :type "Float (single-precision)"))
  ;[1 1 1] On Click - In Hand State
  (`/Engine/EditorBlueprintResources/StandardMacros.Gate` true :!label _label_2
    (:`Exit`
      (`self.K2_TeleportTo` (`KismetMathLibrary.MakeVector` (.x (`.Location` (`GameplayStatics.BreakHitResult` (`PlayerController.GetHitResultUnderCursorByChannel` (`GameplayStatics.GetPlayerController` 0) "TraceTypeQuery1" true)))) (.y (`.Location` (`GameplayStatics.BreakHitResult` (`PlayerController.GetHitResultUnderCursorByChannel` (`GameplayStatics.GetPlayerController` 0) "TraceTypeQuery1" true)))) (.z (`self.K2_GetActorLocation`))) (`SceneComponent.K2_GetComponentRotation` (`self.Card`))))))

(event `CloseOnClickGate`
  ;[1 1 1] On Click - In Hand State
  (goto _label :!via `Close`))

(event `CloseGate`
  ;[1 1 1] On Click - In Hand State
  (goto _label_2 :!via `Close`))

(event `self.Card.OnReleased`
  (params (TouchedComponent :type "PrimitiveComponent Object Reference") (ButtonReleased :type "Key Structure"))
  (switch `/Game/Blueprints/Cards/CardStateEnum` (`self.StateSelection`)
    (:`NewEnumerator1`
      ;[1 1 1] On release - In Hand State
      (`/Engine/EditorBlueprintResources/StandardMacros.Gate` false :!label _label_3
        (:`Exit`
          (set `self.MouseRelased` true)
          (`self.CloseGate`))))
    (:`NewEnumerator2`
      (`self.Release Click - Board State`))))

(event `CloseOnRelaseGate`
  ;[1 1 1] On release - In Hand State
  (`self.StopHover`)
  (goto _label_3 :!via `Close`))

(fn `End Hover`
  (`self.K2_TeleportTo` (- (`SceneComponent.K2_GetComponentLocation` (`self.Card`)) (0.0 -20.0 30.0)) (`self.K2_GetActorRotation`))
  (`SceneComponent.SetWorldScale3D` (`self.DefaultSceneRoot`) (0.3 0.3 0.3)))

(fn `On Click - Boad State`
  (bind (_bblockinghit _binitialoverlap _time _distance _location _impactpoint _normal _impactnormal _physmat _hitactor) (`GameplayStatics.BreakHitResult` (`PlayerController.GetHitResultUnderCursorByChannel` (`GameplayStatics.GetPlayerController` 0) "TraceTypeQuery1" true)))
  (if (== (`GameplayStatics.GetObjectClass` _hitactor) "/Game/Blueprints/Cards/BaseCard.BaseCard_C")
    (bind _asbase_card (cast `/Game/Blueprints/Cards/BaseCard` _hitactor))
    (`/Game/Blueprints/GameState/Card_GameMode.Combat Check 1` (cast `/Game/Blueprints/GameState/Card_GameMode` (`GameplayStatics.GetGameMode`) :!pure true) (`/Game/Blueprints/Cards/BaseCard.Att_Value` _asbase_card) (`/Game/Blueprints/Cards/BaseCard.Def_Value` _asbase_card) _asbase_card)))

(fn `On Hover`
  (`self.K2_TeleportTo` (+ (`SceneComponent.K2_GetComponentLocation` (`self.Card`)) (0.0 -20.0 30.0)) (`self.K2_GetActorRotation`))
  (`SceneComponent.SetWorldScale3D` (`self.DefaultSceneRoot`) (0.5 0.5 0.5)))

(fn `Release Click - Board State`
  (bind (_bblockinghit _binitialoverlap _time _distance _location _impactpoint _normal _impactnormal _physmat _hitactor) (`GameplayStatics.BreakHitResult` (`PlayerController.GetHitResultUnderCursorByChannel` (`GameplayStatics.GetPlayerController` 0) "TraceTypeQuery1" true)))
  (if (== (`GameplayStatics.GetObjectClass` _hitactor) "/Game/Blueprints/Cards/BaseCard.BaseCard_C")
    (bind _asbase_card (cast `/Game/Blueprints/Cards/BaseCard` _hitactor))
    (`/Game/Blueprints/GameState/Card_GameMode.Combat Check 2` (cast `/Game/Blueprints/GameState/Card_GameMode` (`GameplayStatics.GetGameMode`) :!pure true) (`/Game/Blueprints/Cards/BaseCard.Att_Value` _asbase_card) (`/Game/Blueprints/Cards/BaseCard.Def_Value` _asbase_card) _asbase_card)))

(fn `UpdateValues`
  ;[1 1 1] Sets card value based on database
  (`TextRenderComponent.K2_SetText` (`self.Card Name`) (`self.Title_Text`))
  (`TextRenderComponent.K2_SetText` (`self.Att`) (`KismetTextLibrary.Conv_IntToText` (`self.Att_Value`)))
  (`TextRenderComponent.K2_SetText` (`self.Def`) (`KismetTextLibrary.Conv_IntToText` (`self.Def_Value`)))
  (`TextRenderComponent.K2_SetText` (`self.ManaCost`) (`KismetTextLibrary.Conv_IntToText` (`self.ManaCost_Value`))))

(fn `UserConstructionScript`
  ;[1 1 1] Sets starting values
  (`TextRenderComponent.K2_SetText` (`self.Card Name`) (`self.Title_Text`))
  (`TextRenderComponent.K2_SetText` (`self.Att`) (`KismetTextLibrary.Conv_IntToText` (`self.Att_Value`)))
  (`TextRenderComponent.K2_SetText` (`self.Def`) (`KismetTextLibrary.Conv_IntToText` (`self.Def_Value`)))
  (`TextRenderComponent.K2_SetText` (`self.ManaCost`) (`KismetTextLibrary.Conv_IntToText` (`self.ManaCost_Value`))))