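; BaseCard is a base card Blueprint that displays a card's title, attack, defense and mana cost.
; Its construction script copies the title, attack, defense and mana values into their matching text elements, converting the numeric stats to text.
; The displayed text therefore follows the values whenever the construction script runs.
; A comment marks the script for refactoring once the feature is complete.
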(fn `UserConstructionScript`
  ;[1 1 1] Refactor when complete feature
  (`TextRenderComponent.K2_SetText` (`self.Card Name`) (`self.Title_Text`))
  (`TextRenderComponent.K2_SetText` (`self.Att`) (`KismetTextLibrary.Conv_IntToText` (`self.Att_Value`)))
  (`TextRenderComponent.K2_SetText` (`self.Def`) (`KismetTextLibrary.Conv_IntToText` (`self.Def_Value`)))
  (`TextRenderComponent.K2_SetText` (`self.ManaCost`) (`KismetTextLibrary.Conv_IntToText` (`self.ManaCost_Value`))))