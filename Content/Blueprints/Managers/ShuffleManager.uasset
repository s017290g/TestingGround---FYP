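; ShuffleManager spawns the AI's card deck from AI_Card_Data_Table when play begins.
; It shuffles a copy of the row names into CardsInDeck, but the spawn loop iterates the unshuffled names.
; Each row becomes a scaled AI_Cards actor at the deck position, fed via SetCardData, with AllCards refreshed every iteration.
; An unconnected older chain would assign shuffled names to existing cards while spawning BaseCard actors.
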(event `self.ReceiveBeginPlay`
  ;[1 1 1] Get cards from the data table
  (bind _outrownames (`DataTableFunctionLibrary.GetDataTableRowNames` "/Game/Blueprints/Cards/AI_Card_Data_Table.AI_Card_Data_Table"))
  (bind _output_get (set `self.Cards In Deck` _outrownames))
  (`KismetArrayLibrary.Array_Shuffle` _output_get)
  ;[1 1 1] For each card in deck, loop though and set the cards data values, when done, set the game state to deal to hand
  (for _array_element _outrownames
    (bind _returnvalue (`|SpawnActorFromClass` "/Game/Blueprints/Cards/AI_Cards.AI_Cards_C" (`self.SpawnPositionForDeck`) "AlwaysSpawn" "OverrideRootScale" null null))
    (`SceneComponent.SetWorldScale3D` (`/Game/Blueprints/Cards/AI_Cards.DefaultSceneRoot` _returnvalue) (`self.Scale for Grave / Deck`))
    (bind _outactors (`GameplayStatics.GetAllActorsOfClass` "/Game/Blueprints/Cards/AI_Cards.AI_Cards_C"))
    (set `self.AllCards` _outactors)
    (`/Game/Blueprints/Cards/AI_Cards.Set Card Data` _returnvalue _array_element)))

(fn `UserConstructionScript`)