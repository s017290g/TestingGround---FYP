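; DrawManager deals a random hand of cards in front of the player when play begins.
; It gathers every BaseCard actor in the level, shuffles them, and teleports those in a configurable index range into a row.
; The row starts at a hard-coded offset from the player pawn and advances by a fixed step per card.
; Card roll is taken from the pawn's pitch.
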(event `self.ReceiveBeginPlay`
  ;[1 1 1] For the love of all that is holy, change this
  (bind _outactors (`GameplayStatics.GetAllActorsOfClass` "/Game/Blueprints/Cards/BaseCard.BaseCard_C"))
  (bind _output_get (set `self.AllCards` _outactors))
  (`KismetArrayLibrary.Array_Shuffle` _output_get)
  (set `self.CardStartLoc` (+ (`self.K2_GetActorLocation` (`GameplayStatics.GetPlayerPawn` 0)) (-150.0 200.0 -450.0)))
  (set `self.CardRotation` (`KismetMathLibrary.MakeRotator` (.pitch (`SceneComponent.K2_GetComponentRotation` (`Actor.RootComponent` (`GameplayStatics.GetPlayerPawn` 0))))))
  (for _index (range (`self.StartingNo`) (+ (`self.EndingNo`) 1))
    (set `self.AmountOfDrawnCards` _index)
    (`self.K2_TeleportTo` (`|GetArrayItem` (`self.AllCards`) (`self.AmountOfDrawnCards`)) (`self.CardStartLoc`) (`self.CardRotation`))
    (set `self.CardStartLoc` (+ (`self.CardStartLoc`) (`self.CardOffsetToNext`)))))

(fn `UserConstructionScript`)