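; AI_Manager builds and shuffles the AI's card deck when play begins.
; Shuffle spawns one AI_Cards actor per AI_Card_Data_Table row at an offset from its root, scales it and passes it the row name.
; Draw then gathers all AI_Cards actors into AllCards and shuffles that array.
; The loop that would teleport drawn cards into a line is disconnected, and AITrigger is an empty event.
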(event `self.ReceiveBeginPlay`
  (`|ExecutionSequence`
    (:`then_0`
      (`self.Shuffle`))
    (:`then_1`
      (`self.Draw`))))

(event `AI Trigger`)

(fn `Draw`
  (`|ExecutionSequence`
    (:`then_0`
      (bind _outactors (`GameplayStatics.GetAllActorsOfClass` "/Game/Blueprints/Cards/AI_Cards.AI_Cards_C"))
      (bind _output_get (set `self.AllCards` _outactors))
      (`KismetArrayLibrary.Array_Shuffle` _output_get))))

(fn `Shuffle`
  (locals (`Scale For Gave / Deck` :type "Vector Structure" :default (0.3 0.3 0.3)))
  (bind _outrownames (`DataTableFunctionLibrary.GetDataTableRowNames` "/Game/Blueprints/Cards/AI_Card_Data_Table.AI_Card_Data_Table"))
  (bind _output_get (set `self.Cards In Deck` _outrownames))
  (`KismetArrayLibrary.Array_Shuffle` _output_get)
  (for _array_element _outrownames
    (bind _returnvalue (`|SpawnActorFromClass` "/Game/Blueprints/Cards/AI_Cards.AI_Cards_C" (`KismetMathLibrary.MakeTransform` (+ (`SceneComponent.K2_GetComponentLocation` (`self.DefaultSceneRoot`)) (.location (`self.Spawn Transform For Deck`))) (struct :`Roll` 90.0) (1.0 1.0 1.0)) "AlwaysSpawn" "OverrideRootScale" null null))
    (`SceneComponent.SetWorldScale3D` (`/Game/Blueprints/Cards/AI_Cards.DefaultSceneRoot` _returnvalue) (`local.Scale For Gave / Deck`))
    (bind _outactors (`GameplayStatics.GetAllActorsOfClass` "/Game/Blueprints/Cards/AI_Cards.AI_Cards_C"))
    (set `self.AllCards` _outactors)
    (`/Game/Blueprints/Cards/AI_Cards.Set Card Data` _returnvalue _array_element)))

(fn `UserConstructionScript`)