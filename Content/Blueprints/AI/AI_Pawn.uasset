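; AI opponent pawn for a card game that takes the enemy turn by playing a card from its hand.
; BeginEnemyTurn scans the hand for a card within its mana, breaks the loop through a custom event, then moves that card to an offset from its old location and removes it from the hand.
; It then sets the next state on Card_GameMode and triggers the state switch.
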(event `BreakLoop`
  (bind _ascard_game_mode (cast `/Game/Blueprints/GameState/Card_GameMode` (`GameplayStatics.GetGameMode`) :!pure true))
  ;[1 1 1] Card Placement
  (goto _label :!via `Break`))

(event `Begin Enemy Turn`
  (bind _ascard_game_mode (cast `/Game/Blueprints/GameState/Card_GameMode` (`GameplayStatics.GetGameMode`) :!pure true))
  ;[1 1 1] Card Placement
  (for _array_element (`self.Cards in hand array`) :!label _label
    (if (<= (`/Game/Blueprints/Cards/AI_Cards.ManaCost_Value` _array_element) (`self.Mana`))
      (`self.BreakLoop`)
      (`self.K2_SetActorTransform` _array_element (`KismetMathLibrary.MakeTransform` (+ (`/Game/Blueprints/Cards/AI_Cards.OldLoc` _array_element) (0.0 150.0 -40.0)) (struct :`Roll` -90.0) (0.3 0.3 0.3)) false false)
      (`KismetArrayLibrary.Array_RemoveItem` (`self.Cards in hand array`) _array_element)))
  (set `/Game/Blueprints/GameState/Card_GameMode.StateSelection` "NewEnumerator2" _ascard_game_mode)
  (`/Game/Blueprints/GameState/Card_GameMode.SwitchGameStateEnum` _ascard_game_mode))

(fn `UserConstructionScript`)