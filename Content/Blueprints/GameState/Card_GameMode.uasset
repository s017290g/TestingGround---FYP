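; Game mode for a card game that runs turn phases through a state switch, with most phases still debug-print stubs.
; Shuffle spawns a BaseCard per data table row, assigning shuffled row data to all but the last, then switches to Deal to Hand.
; Dealing reshuffles the card actors and teleports an index range into an evenly offset line positioned relative to the player pawn.
; Untap only sorts cards by owning player for debug prints.
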(event `self.ReceiveBeginPlay`
  ;[1 1 1] Switch for game state
  (switch `/Game/Blueprints/GameState/GameStatesEnum` (`self.StateSelection`) :!label _label
    (:`NewEnumerator12`
      (`self.Shuffle Function`)
      (`KismetSystemLibrary.PrintString` "Hello"))
    (:`NewEnumerator13`
      (`self.Draw Function`)
      (`KismetSystemLibrary.PrintString` "DONE"))
    (:`NewEnumerator2`
      (`KismetSystemLibrary.PrintString` "Upkeep"))
    (:`NewEnumerator1`
      (`KismetSystemLibrary.PrintString` "Untap")
      (bind _outactors (`GameplayStatics.GetAllActorsOfClass` "/Game/Blueprints/Cards/BaseCard.BaseCard_C"))
      (for _array_element _outactors
        (bind _asbase_card (cast `/Game/Blueprints/Cards/BaseCard` _array_element))
        (if (`/Game/Blueprints/Cards/BaseCard.IsPlayer1` _asbase_card)
          (`KismetSystemLibrary.PrintString` "Do Player 1 Stuff")
          (else
            (`KismetSystemLibrary.PrintString` "Do Player 2 Stuff")))))
    (:`NewEnumerator3`
      (`KismetSystemLibrary.PrintString` "Draw"))
    (:`NewEnumerator4`
      (`KismetSystemLibrary.PrintString` "MainPhase"))
    (:`NewEnumerator11`
      (`KismetSystemLibrary.PrintString` "Combat"))
    (:`NewEnumerator6`
      (`KismetSystemLibrary.PrintString` "EnemyTurn"))
    (:`NewEnumerator8`
      (`KismetSystemLibrary.PrintString` "PlayerLose"))
    (:`NewEnumerator9`
      (`KismetSystemLibrary.PrintString` "PlayerWin"))))

(event `Custom Event Trigger`
  ;[1 1 1] Switch for game state
  (goto _label))

(fn `Draw Function`
  (bind _outactors (`GameplayStatics.GetAllActorsOfClass` "/Game/Blueprints/Cards/BaseCard.BaseCard_C"))
  (bind _output_get (set `self.AllCards` _outactors))
  (`KismetArrayLibrary.Array_Shuffle` _output_get)
  (set `self.CardStartLoc` (+ (`self.K2_GetActorLocation` (`GameplayStatics.GetPlayerPawn` 0)) (-150.0 200.0 -450.0)))
  (set `self.CardRotation` (`KismetMathLibrary.MakeRotator` (.pitch (`SceneComponent.K2_GetComponentRotation` (`Actor.RootComponent` (`GameplayStatics.GetPlayerPawn` 0))))))
  (for _index (range (`self.StartingNo`) (+ (`self.EndingNo`) 1))
    (set `self.AmountOfDrawnCards` _index)
    (`self.K2_TeleportTo` (`|GetArrayItem` (`self.AllCards`) (`self.AmountOfDrawnCards`)) (`self.CardStartLoc`) (`self.CardRotation`))
    (set `self.CardStartLoc` (+ (`self.CardStartLoc`) (`self.CardOffsetToNext`)))))

(fn `Shuffle Function`
  (bind _outrownames (`DataTableFunctionLibrary.GetDataTableRowNames` "/Game/Blueprints/Cards/Card_Data_Table.Card_Data_Table"))
  (bind _output_get (set `self.Cards In Deck` _outrownames))
  (`KismetArrayLibrary.Array_Shuffle` _output_get)
  (for (_ _array_index) _outrownames
    (bind _returnvalue (`|SpawnActorFromClass` "/Game/Blueprints/Cards/BaseCard.BaseCard_C" (`self.SpawnPositionForDeck`) "AlwaysSpawn" "OverrideRootScale" null null))
    (bind _outactors (`GameplayStatics.GetAllActorsOfClass` "/Game/Blueprints/Cards/BaseCard.BaseCard_C"))
    (set `self.AllCards` _outactors)
    (if (>= _array_index (- (`KismetArrayLibrary.Array_Length` (`self.Cards In Deck`)) 1))
      (set `self.StateSelection` "NewEnumerator13")
      (`self.Custom Event Trigger`)
      (else
        (`/Game/Blueprints/Cards/BaseCard.Set Card Data` _returnvalue (`|GetArrayItem` (`self.Cards In Deck`) (`self.Current Array Index`)))
        (`/Engine/EditorBlueprintResources/StandardMacros.IncrementInt` (`self.Current Array Index`))))))

(fn `UserConstructionScript`)