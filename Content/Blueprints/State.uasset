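; State Blueprint that cycles through the phases of a card-game style turn, from Upkeep through Untap, Draw, Main Phase, End Step and Enemy Turn.
; BeginPlay enters a switch on the StateSelection enum, where each phase prints its name, waits on a fixed delay, then sets the next phase.
; FireEvent calls itself after each step, so the cycle loops endlessly on a timer, with no gameplay logic or player input.
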(event `FireEvent`
  (switch `/Game/Blueprints/GameStatesEnum` (`self.StateSelection`) :!label _label
    (:`NewEnumerator2`
      (`KismetSystemLibrary.PrintString` "Upkeep")
      (`KismetSystemLibrary.Delay` 1.5)
      (set `self.StateSelection` "NewEnumerator1"))
    (:`NewEnumerator1`
      (`KismetSystemLibrary.PrintString` "Untap")
      (`KismetSystemLibrary.Delay` 1.5)
      (set `self.StateSelection` "NewEnumerator3"))
    (:`NewEnumerator3`
      (`KismetSystemLibrary.PrintString` "Draw")
      (`KismetSystemLibrary.Delay` 1.5)
      (set `self.StateSelection` "NewEnumerator4"))
    (:`NewEnumerator4`
      (`KismetSystemLibrary.PrintString` "MainPhase")
      (`KismetSystemLibrary.Delay` 1.5)
      (set `self.StateSelection` "NewEnumerator5"))
    (:`NewEnumerator5`
      (`KismetSystemLibrary.PrintString` "EndStep")
      (`KismetSystemLibrary.Delay` 1.5)
      (set `self.StateSelection` "NewEnumerator6"))
    (:`NewEnumerator6`
      (`KismetSystemLibrary.PrintString` "EnemyTurn")
      (`KismetSystemLibrary.Delay` 1.5)
      (set `self.StateSelection` "NewEnumerator2")))
  (`self.FireEvent`))

(event `self.ReceiveBeginPlay`
  (goto _label))

(fn `UserConstructionScript`)